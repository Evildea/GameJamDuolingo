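; MenuLight is a light actor, likely for a menu scene, that flashes a point light and has a hum sound.
; BeginPlay spawns the LightHum sound at the actor's location and stores it in HumSound.
; While Finished is true, Tick calls Play on the LightFlash timeline, whose scaled track drives light intensity.
; The timeline sets Finished to true on completion, and nothing here clears it.
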(event EventBeginPlay
  (bind _returnvalue (Audio|SpawnSoundatLocation (Variables|Default|GetLightHum) (Transformation|GetActorLocation) "0, 0, 0" 1.0 1.0 0.0 0 0))
  (Variables|Default|SetHumSound _returnvalue))

(event EventTick
  (params (DeltaSeconds :type Float%20%28single-precision%29))
  (if (Variables|Default|GetFinished)
    (bind _newtrack_0 (Timeline|LightFlash Play)
      (:Update
        (Rendering|Components|Light|SetIntensity (Variables|Default|GetPointLight) (* _newtrack_0 5e+03)))
      (:Finished
        (Variables|Default|SetFinished true)))))

(fn ConstructionScript)