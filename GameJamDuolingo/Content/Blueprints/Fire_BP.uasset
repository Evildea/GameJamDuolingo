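; Fire actor that provides a crackling sound and a flickering point light.
; BeginPlay plays the attenuated crackling sound once at the actor's location.
; Tick restarts the Flicker timeline whenever State is idle, and each update scales the curve value into the light's intensity.
; The timeline's Finished output resets State, so the flicker repeats continuously.
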(event EventTick
  (params (DeltaSeconds :type Float%20%28single-precision%29))
  (if (== (Variables|Default|GetState) 0)
    (Variables|Default|SetState 1)
    (bind _newtrack_0 (Timeline|Flicker PlayFromStart)
      (:Update
        (Rendering|Components|Light|SetIntensity (Variables|Default|GetPointLight) (* _newtrack_0 5e+02)))
      (:Finished
        (Variables|Default|SetState 0)))
    (else
      (Timeline|Flicker Play))))

(event EventBeginPlay
  (Audio|PlaySoundatLocation "/Game/Sounds/DuoFootsteps/CracklingFire.CracklingFire" (Transformation|GetActorLocation) "0, 0, 0" 1.0 1.0 0.0 "/Game/Sounds/LightAttenuation.LightAttenuation" 0 0))

(fn ConstructionScript)