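; Mobile_BP is an actor that acts as a proximity-triggered win point for the player.
; Each Tick it checks the distance to the player pawn and shows its Widget component at mid range, hiding it when very close or far away.
; At close range it creates a WinWidget and adds it to the viewport, using an IsCreated flag so this happens only once.
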(event EventTick
  (params (DeltaSeconds :type Float%20%28single-precision%29))
  (bind _returnvalue (Game|Player|GetPlayerPawn 0))
  (bind _widget (Variables|Default|GetWidget))
  (bind _returnvalue_2 (Transformation|GetDistanceTo _returnvalue))
  (Utilities|FlowControl|Sequence
    (:then_0
      (if (and (<= _returnvalue_2 9e+02) (> _returnvalue_2 1e+02))
        (Rendering|SetVisibility _widget true false)
        (else
          (Rendering|SetVisibility _widget false false))))
    (:then_1
      (if (and (<= _returnvalue_2 1e+02) (not (Variables|Default|GetisCreated)))
        (bind _returnvalue_3 (UserInterface|CreateWidget "/Game/UI/WinWidget.WinWidget_C" (Game|GetPlayerController 0)))
        (UserInterface|Viewport|AddtoViewport _returnvalue_3 0)
        (Variables|Default|SetisCreated true)))))

(fn ConstructionScript)