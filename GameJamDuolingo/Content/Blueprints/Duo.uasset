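; Duo is a stalking enemy that, after a startup delay, walks to an offset waypoint, then chases the player.
; A Tick-driven Delay paces the chase, repeatedly raising walk speed, replaying whispers once finished and triggering nearby footsteps with proximity-scaled camera shake.
; Overlapping its CaptureSphere with the FirstPersonCharacter blends the view to Duo and shows the death widget.
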(event OnComponentBeginOverlap(CaptureSphere)
  (params (OverlappedComponent :type Primitive%20Component%20Object%20Reference) (OtherActor :type Actor%20Object%20Reference) (OtherComp :type Primitive%20Component%20Object%20Reference) (OtherBodyIndex :type Integer) (bFromSweep :type Boolean) (SweepResult :type Hit%20Result%20Structure%20%28by%20ref%29))
  (Utilities|Casting|CastToFirstPersonCharacter OtherActor)
  (Game|Player|SetViewTargetwithBlend (Game|GetPlayerController 0) self 0.25 "VTBlend_Linear" 0.0 false)
  (bind _returnvalue (UserInterface|CreateWidget "/Game/UI/DeathWidget.DeathWidget_C" (Game|GetPlayerController 0)))
  (UserInterface|Viewport|AddtoViewport _returnvalue 0))

(event EventBeginPlay
  (Utilities|FlowControl|Delay 8.5)
  (Variables|Default|SetDefault%20Location (Transformation|GetActorLocation))
  (Variables|Default|SetActivated true))

(event EventTick
  (params (DeltaSeconds :type Float%20%28single-precision%29))
  (bind _charactermovement (Variables|Character|GetCharacterMovement))
  (if (Variables|Default|GetActivated)
    (if (Variables|Default|GetFirst%20Target%20Complete)
      (AI|Navigation|SimpleMovetoActor (Pawn|GetController) (Game|Player|GetPlayerPawn 0))
      (Utilities|FlowControl|Delay 0.5)
      (CallFunction|Footsteps)
      (CallFunction|Whispers)
      (Variables|/Script/Engine.CharacterMovementComponent|SetMaxWalkSpeed _charactermovement (+ (Variables|/Script/Engine.CharacterMovementComponent|GetMaxWalkSpeed _charactermovement) 1.0))
      (else
        (AI|Navigation|SimpleMovetoLocation (Pawn|GetController) (+ (Variables|Default|GetDefault%20Location) (Variables|Designer|GetFirst%20Walk%20To%20Target)))
        (Utilities|FlowControl|Delay (Variables|Designer|GetFirst%20Walk%20To%20Duration))
        (Variables|Default|SetFirst%20Target%20Complete true)))))

(fn ConstructionScript)

(fn Footsteps
  (bind _returnvalue (Game|Player|GetPlayerPawn 0))
  (bind _self self)
  (bind _shake_distance (Variables|Designer|GetShake%20Distance))
  (bind _returnvalue_2 (Transformation|GetDistanceTo _returnvalue _self))
  (if (<= _returnvalue_2 _shake_distance)
    (Class|PlayerController|ClientPlayCameraShake (Game|GetPlayerController 0) (Variables|Designer|GetCamera%20Shake) (* (/ 1.0 _shake_distance) (- _shake_distance _returnvalue_2)) "CameraLocal" "0, 0, 0")
    (Audio|SpawnSoundatLocation "/Game/Sounds/DuoFootsteps/FootstepCue.FootstepCue" (Transformation|GetActorLocation) "0, 0, 0" 1.0 1.0 0.0 0 0)))

(fn Whispers
  (Utilities|IsValid (Variables|Default|GetWhisperComponent)
    (:Is%20Valid
      (if (not (Audio|Components|Audio|IsPlaying (Variables|Default|GetWhisperComponent)))
        (bind _returnvalue (Audio|SpawnSoundatLocation (Variables|Default|GetWhisperCue) (Transformation|GetActorLocation) "0, 0, 0" 1.0 1.0 0.0 0 0 :!label _label))
        (Variables|Default|SetWhisperComponent _returnvalue)))
    (:Is%20Not%20Valid
      (goto _label))))